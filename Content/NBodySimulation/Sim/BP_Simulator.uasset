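; BP_Simulator is an N-body simulation actor that sets up the camera rig, plane and test input.
; Construction positions CameraArm and Plane; BeginPlay adds the input mapping context and calls GetCameraValues after a short delay.
; IA_AXIS writes InputVector, but the Plane movement that reads it is disconnected.
; NewFunction draws a debug box and corner spheres from 2D bounds; its SceneBounds quadrant call is also disconnected.
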(event `self.ReceiveBeginPlay`
  (`|ExecutionSequence`
    (:`then_0`
      (`EnhancedInputSubsystemInterface.AddMappingContext` (pcsubsystem `EnhancedInputLocalPlayerSubsystem` (`GameplayStatics.GetPlayerController` 0)) "/Game/Developers/IMC_Test.IMC_Test" 0 (struct)))
    (:`then_1`
      (`KismetSystemLibrary.Delay` 1.0)
      (`self.GetCameraValues`))))

(event `EnhancedInput|/Game/Developers/IA_AXIS`
  (params (ActionValue :type "Vector2D Structure") (ElapsedSeconds :type "Float (double-precision)") (TriggeredSeconds :type "Float (double-precision)") (InputAction :type "InputAction Object Reference" :default "/Game/Developers/IA_AXIS.IA_AXIS"))
  (bind (_x _y) (`KismetMathLibrary.BreakVector2D` ActionValue))
  (:`Triggered`
    (set `self.InputVector` (`KismetMathLibrary.MakeVector` _x _y)))
  (:`Canceled`
    (set `self.InputVector` (0.0 0.0 0.0) :!label _label))
  (:`Completed`
    (goto _label)))

(event `self.ReceiveTick`
  (params (DeltaSeconds :type "Float (single-precision)")))

(fn `NewFunction`
  (params (Min :type "Vector2D Structure") (Max :type "Vector2D Structure"))
  (bind (_center _extents) (`BodySimulatorFunctionLibrary.GetBoxBounds` (`KismetMathLibrary.MakeBox2D` Min Max)))
  (`KismetSystemLibrary.DrawDebugBox` (`KismetMathLibrary.Conv_Vector2DToVector` _center) (`KismetMathLibrary.Conv_Vector2DToVector` _extents) (struct :`R` 1.0 :`B` 0.250507 :`A` 1.0) (struct) 0.0 22.0)
  (`KismetSystemLibrary.DrawDebugSphere` (`KismetMathLibrary.Conv_Vector2DToVector` Min))
  (`KismetSystemLibrary.DrawDebugSphere` (`KismetMathLibrary.Conv_Vector2DToVector` Max) 100.0 12 (struct :`R` 0.644285 :`B` 1.0 :`A` 1.0)))

(fn `UserConstructionScript`
  (`SceneComponent.K2_SetRelativeLocation` (`self.CameraArm`) (1648.5 2500.0 0.0) false false)
  (`SceneComponent.K2_SetWorldLocation` (`self.Plane`) (0.0 0.0 0.0) false false))