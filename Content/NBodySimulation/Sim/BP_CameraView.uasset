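; BP_CameraView is a possessable test actor in the N-body simulation that flies a Plane across the camera view with screen-edge wraparound.
; Shortly after possession it deprojects the viewport corners to world bounds and picks a random 3D direction.
; Tick moves the Plane at constant speed, and NewFunction wraps X and Y to the opposite bound, leaving Z untouched.
; BeginPlay adds IMC_Test, but no input actions are handled here.
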(event `self.ReceiveBeginPlay`
  (`EnhancedInputSubsystemInterface.AddMappingContext` (pcsubsystem `EnhancedInputLocalPlayerSubsystem` (`GameplayStatics.GetPlayerController` 0)) "/Game/Developers/IMC_Test.IMC_Test" 0 (struct)))

(event `self.ReceivePossessed`
  (params (NewController :type "Controller Object Reference"))
  (bind (_returnvalue_x _returnvalue_y) (`KismetMathLibrary.BreakVector2D` (`WidgetLayoutLibrary.GetViewportSize`)))
  (`KismetSystemLibrary.Delay` 0.2)
  (bind _output_get (set `self.TopLeft` (`GameplayStatics.DeprojectScreenToWorld` (`GameplayStatics.GetPlayerController` 0) (0.0 0.0))))
  (set `self.BottomRight` (`GameplayStatics.DeprojectScreenToWorld` (`GameplayStatics.GetPlayerController` 0) (`KismetMathLibrary.MakeVector2D` _returnvalue_x _returnvalue_y)))
  (set `self.InputVector` (`KismetMathLibrary.RandomUnitVector`)))

(event `self.ReceiveTick`
  (params (DeltaSeconds :type "Float (single-precision)"))
  (bind _plane (`self.Plane`))
  (`SceneComponent.K2_AddWorldOffset` (`self.Plane`) (* (`self.InputVector`) DeltaSeconds 11111.0) false false)
  (bind _adjustedposition (`self.NewFunction` (`SceneComponent.K2_GetComponentLocation` _plane)))
  (`SceneComponent.K2_SetWorldLocation` _plane _adjustedposition false true))

(fn `NewFunction`
  (params (InVec :type "Vector Structure"))
  (returns (AdjustedPosition :type "Vector Structure"))
  (locals (AdjustedX :type "Float (double-precision)") (AdjustedY :type "Float (double-precision)"))
  (bind _x (.x InVec))
  (bind _y (.y InVec))
  (bind (_bottomright_x _bottomright_y) (`KismetMathLibrary.BreakVector` (`self.BottomRight`)))
  (bind _x_2 (.x (`self.TopLeft`)))
  (bind _y_2 (.y (`self.TopLeft`)))
  (bind _x_3 (.x (`self.BottomRight`)))
  (`|ExecutionSequence`
    (:`then_0`)
    (:`then_1`
      (if (> _x (+ _x_2 0.0))
        (set `local.AdjustedX` _x_3)
        (elif (< _x _x_3)
          (set `local.AdjustedX` _x_2)
          (else
            (set `local.AdjustedX` _x)))))
    (:`then_2`
      (if (< _y _y_2)
        (set `local.AdjustedY` _bottomright_y)
        (elif (> _y _bottomright_y)
          (set `local.AdjustedY` _y_2)
          (else
            (set `local.AdjustedY` _y)))))
    (:`then_3`
      (return (`KismetMathLibrary.MakeVector` (`local.AdjustedX`) (`local.AdjustedY`) (.z InVec))))))

(fn `UserConstructionScript`)